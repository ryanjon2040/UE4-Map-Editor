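; Placeable blue building for the map editor example, assembled from modular 400x400 wall and floor meshes.
; Its construction script assigns four plain walls, one door wall and one floor to six static mesh components.
; It runs the parent construction script last, so any parent setup sees the meshes already assigned.
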(fn `UserConstructionScript`
  (`|ExecutionSequence`
    (:`then_0`
      (`StaticMeshComponent.SetStaticMesh` (`self.StaticMesh1`) "/Game/StarterContent/Architecture/Wall_400x400.Wall_400x400"))
    (:`then_1`
      (`StaticMeshComponent.SetStaticMesh` (`self.StaticMesh2`) "/Game/StarterContent/Architecture/Wall_Door_400x400.Wall_Door_400x400"))
    (:`then_2`
      (`StaticMeshComponent.SetStaticMesh` (`self.StaticMesh3`) "/Game/StarterContent/Architecture/Wall_400x400.Wall_400x400"))
    (:`then_3`
      (`StaticMeshComponent.SetStaticMesh` (`self.StaticMesh4`) "/Game/StarterContent/Architecture/Wall_400x400.Wall_400x400"))
    (:`then_4`
      (`StaticMeshComponent.SetStaticMesh` (`self.StaticMesh5`) "/Game/StarterContent/Architecture/Wall_400x400.Wall_400x400"))
    (:`then_5`
      (`StaticMeshComponent.SetStaticMesh` (`self.StaticMesh6`) "/Game/StarterContent/Architecture/Floor_400x400.Floor_400x400"))
    (:`then_6`
      (`parent.UserConstructionScript`))))