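; Base building Blueprint for the map editor example, supporting a placement-style preview mode and player-chosen recoloring.
; Construction creates a dynamic material instance, which SetMaterial applies to five static meshes, or swaps for a preview material.
; Preview mode also disables actor collision.
; Clicking the selection box sends the building and its color options to the player controller; ApplyColor then updates the instance's Color parameter.
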(event `PreviewMode`
  (params (bIsInPreviewMode :type Boolean :default false))
  (`self.SetActorEnableCollision` (not bIsInPreviewMode))
  (`self.SetMaterial` bIsInPreviewMode))

(event `self.SelectionBox.OnClicked`
  (params (TouchedComponent :type "PrimitiveComponent Object Reference"))
  (message `/Game/MapEditorExample/Blueprints/Interfaces/BPI_HUD_Controller.PopulateColorButtons` (`GameplayStatics.GetPlayerController` 0) (`self.STRUCT_Colors`) self))

(event `self.ApplyColor`
  (params (ColorToApply :type "Object.LinearColor Structure"))
  (`MaterialInstanceDynamic.SetVectorParameterValue` (`self.BuildingMat`) "Color" ColorToApply)
  (`self.SetMaterial` false))

(fn `SetMaterial`
  (params (bPreviewMode :type Boolean :default false))
  (`PrimitiveComponent.SetMaterial` (`self.StaticMesh1`) 0 (select `bool` bPreviewMode :`false` (`self.BuildingMat`) :`true` "/Game/MapEditorExample/Materials/M_Preview.M_Preview" :!type "MaterialInterface Object Reference"))
  (`PrimitiveComponent.SetMaterial` (`self.StaticMesh2`) 0 (select `bool` bPreviewMode :`false` (`self.BuildingMat`) :`true` "/Game/MapEditorExample/Materials/M_Preview.M_Preview" :!type "MaterialInterface Object Reference"))
  (`PrimitiveComponent.SetMaterial` (`self.StaticMesh3`) 0 (select `bool` bPreviewMode :`false` (`self.BuildingMat`) :`true` "/Game/MapEditorExample/Materials/M_Preview.M_Preview" :!type "MaterialInterface Object Reference"))
  (`PrimitiveComponent.SetMaterial` (`self.StaticMesh4`) 0 (select `bool` bPreviewMode :`false` (`self.BuildingMat`) :`true` "/Game/MapEditorExample/Materials/M_Preview.M_Preview" :!type "MaterialInterface Object Reference"))
  (`PrimitiveComponent.SetMaterial` (`self.StaticMesh5`) 0 (select `bool` bPreviewMode :`false` (`self.BuildingMat`) :`true` "/Game/MapEditorExample/Materials/M_Preview.M_Preview" :!type "MaterialInterface Object Reference"))
  (return))

(fn `UserConstructionScript`
  (bind _returnvalue (`KismetMaterialLibrary.CreateDynamicMaterialInstance` "/Game/MapEditorExample/Materials/M_BuildingMaster.M_BuildingMaster"))
  (set `self.BuildingMat` _returnvalue)
  (`self.SetMaterial` false))