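; Map editor foliage brush actor that scatters BP_Foliage actors while painting is active.
; StartPainting paints immediately and starts a looping timer that repeats PaintFoliage until StopPainting clears it.
; Each pass spawns a random count, up to MaxFoliageCount, with random yaw and per-axis scale.
; Locations are random points in the brush mesh bounds, vector-projected onto the impact point of an upward sphere trace.
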(event `StartPainting`
  (`self.PaintFoliage`) ; First stroke
  (`KismetSystemLibrary.K2_SetTimer` null "PaintFoliage" 0.2 true))

(event `StopPainting`
  (`KismetSystemLibrary.K2_ClearTimer` null "PaintFoliage"))

(event `PaintFoliage`
  (bind _returnvalue (`self.K2_GetActorLocation`))
  (bind _minscale (`self.MinScale`))
  (bind _maxscale (`self.MaxScale`))
  (bind (_origin _boxextent _sphereradius) (`KismetSystemLibrary.GetComponentBounds` (`self.BrushMesh`)))
  (for _ (range 1 (+ (`KismetMathLibrary.RandomIntegerInRange` 1 (`self.MaxFoliageCount`)) 1))
    (bind _outhit (`KismetSystemLibrary.SphereTraceSingle_NEW` _returnvalue (+ _returnvalue (* (`self.GetActorUpVector`) 100.0)) (/ _sphereradius 2.0) "TraceTypeQuery1"))
    (`|SpawnActorFromClass` "/Game/MapEditorExample/Blueprints/Misc/BP_Foliage.BP_Foliage_C" (`KismetMathLibrary.MakeTransform` (`KismetMathLibrary.ProjectVectorOnToVector` (`KismetMathLibrary.RandomPointInBoundingBox` _origin _boxextent) (`.ImpactPoint` (`GameplayStatics.BreakHitResult` _outhit))) (`KismetMathLibrary.MakeRot` 0.0 (`KismetMathLibrary.RandomFloatInRange` 0.0 360.0)) (`KismetMathLibrary.MakeVector` (`KismetMathLibrary.RandomFloatInRange` _minscale _maxscale) (`KismetMathLibrary.RandomFloatInRange` _minscale _maxscale) (`KismetMathLibrary.RandomFloatInRange` _minscale _maxscale))))))

(fn `UserConstructionScript`)