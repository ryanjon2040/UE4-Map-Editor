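; Player controller for a runtime map editor that places buildings, a player start and foliage, and switches between editing and playing.
; While a gate is open, Tick traces under the mouse to move the active preview or brush, and left click places or paints.
; Interface events drive spawning, building recoloring and deletion through the HUD.
; Play, pause and stop swap between the spawned character and a free-cam or RTS-style editor camera.
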(event `self.SpawnFoliageBrush`
  (bind _returnvalue (`|SpawnActorFromClass` "/Game/MapEditorExample/Blueprints/Misc/BP_PaintBrush.BP_PaintBrush_C" (`KismetMathLibrary.MakeTransform` (0.0 0.0 0.0))))
  (set `self.EditorPaintBrush` _returnvalue)
  (`self.OpenGate`))

(event `self.DeleteActor`
  ;[1 1 1] Interface Event: Delete building
  (`self.K2_DestroyActor` (`self.SelectedBuilding`))
  (`/Game/MapEditorExample/Blueprints/HUD/EditorHUD.RemoveColorButtons` (`self.EditorHUD`)))

(event `self.ReceiveTick`
  (params (DeltaSeconds :type "Float (single-precision)"))
  (bind (_locationx _locationy) (`self.GetMousePosition`))
  (bind _editorpaintbrush (`self.EditorPaintBrush`))
  (bind _deprojectworldlocation (`self.DeprojectWorldLocation`))
  (bind _previewbuilding (`self.PreviewBuilding`))
  (bind _editorplayerstart (`self.EditorPlayerStart`))
  (bind (_worldlocation _worlddirection) (`self.DeprojectScreenPositionToWorld` _locationx _locationy))
  (`|ExecutionSequence`
    (:`then_0`
      (set `self.DeprojectWorldLocation` _worldlocation))
    (:`then_1`
      (set `self.DeprojectWorldDirection` _worlddirection))
    (:`then_2`
      (`/Engine/EditorBlueprintResources/StandardMacros.Gate` true :!label _label
        (:`Exit`
          (bind _outhit (`KismetSystemLibrary.LineTraceSingle` _deprojectworldlocation (+ _deprojectworldlocation (* (`self.DeprojectWorldDirection`) (`self.TraceDistance`))) "TraceTypeQuery1"))
          (bind _output_get (set `self.PreviewBuildingLocation` (`.ImpactPoint` (`GameplayStatics.BreakHitResult` _outhit))))
          (`|ExecutionSequence`
            (:`then_0`
              (`/Engine/EditorBlueprintResources/StandardMacros.IsValid` _previewbuilding
                (:`Is Valid`
                  (`self.K2_SetActorLocation` _previewbuilding _output_get false))))
            (:`then_1`
              (`/Engine/EditorBlueprintResources/StandardMacros.IsValid` _editorplayerstart
                (:`Is Valid`
                  (if (not (`/Game/MapEditorExample/Blueprints/Misc/BP_PlayerStart.bCanBeMoved` _editorplayerstart))
                    (`self.K2_SetActorLocation` _editorplayerstart (`KismetMathLibrary.MakeVector` (.x _output_get) (.y _output_get) (.z (`self.K2_GetActorLocation` _editorplayerstart))) false)))))
            (:`then_2`
              (`/Engine/EditorBlueprintResources/StandardMacros.IsValid` _editorpaintbrush
                (:`Is Valid`
                  (`self.K2_SetActorLocation` _editorpaintbrush _output_get false))))))))))

(event `self.SpawnBuilding`
  (params (BuildingType :type "/Game/MapEditorExample/Blueprints/Enums/EBuildingTypes Enum" :default "NewEnumerator0"))
  ;[1 1 1] Interface Event: Spawns preview building
  (switch `/Game/MapEditorExample/Blueprints/Enums/EBuildingTypes` BuildingType
    (:`NewEnumerator0`
      (`self.SpawnBuildingInWorld` "/Game/MapEditorExample/Blueprints/Buildings/Placeable/BP_Blue_Building.BP_Blue_Building_C" true))
    (:`NewEnumerator1`
      (`self.SpawnBuildingInWorld` "/Game/MapEditorExample/Blueprints/Buildings/Placeable/BP_Red_Building.BP_Red_Building_C" true))))

(event `OpenGate`
  (goto _label :!via `Open`))

(event `CloseGate`
  (goto _label :!via `Close`))

(event `self.ApplyColor`
  (params (ColorToApply :type "Object.LinearColor Structure"))
  ;[1 1 1] Interface Event: Change color on building
  (`/Game/MapEditorExample/Blueprints/Buildings/BP_MasterBuilding.ApplyColor` (`self.SelectedBuilding`) ColorToApply))

(event `self.PopulateColorButtons`
  (params (STRUCT_Colors :type "Array of /Game/MapEditorExample/Blueprints/Enums/STRUCT_ActorColors Structure (by ref)") (Building :type "/Game/MapEditorExample/Blueprints/Buildings/BP_MasterBuilding Object Reference"))
  (bind _editorhud (`self.EditorHUD`))
  ;[1 1 1] Interface Event: Populate color buttons in Actor Details
  (set `self.SelectedBuilding` Building)
  (`/Game/MapEditorExample/Blueprints/HUD/EditorHUD.RemoveColorButtons` _editorhud)
  (for _array_element STRUCT_Colors
    (bind (_color _colorname) (break `/Game/MapEditorExample/Blueprints/Enums/STRUCT_ActorColors` _array_element))
    (`/Game/MapEditorExample/Blueprints/HUD/EditorHUD.AddColorButton` (`self.EditorHUD`) _color _colorname))
  (`/Game/MapEditorExample/Blueprints/HUD/EditorHUD.AddDeleteButton` _editorhud))

(event `self.SpawnPlayerStart`
  ;[1 1 1] Interface Event: Spawn player start
  (`/Engine/EditorBlueprintResources/StandardMacros.IsValid` (`self.EditorPlayerStart`)
    (:`Is Not Valid`
      (bind _returnvalue (`|SpawnActorFromClass` "/Game/MapEditorExample/Blueprints/Misc/BP_PlayerStart.BP_PlayerStart_C" (`KismetMathLibrary.MakeTransform` (0.0 0.0 0.0) (struct) (1.0 1.0 1.0))))
      (set `self.EditorPlayerStart` _returnvalue)
      (`self.OpenGate`))))

(event `Key|LeftMouseButton`
  (bind _editorpaintbrush (`self.EditorPaintBrush`))
  (bind _previewbuilding (`self.PreviewBuilding`))
  (bind _editorplayerstart (`self.EditorPlayerStart`))
  (bind _editorplayerstart_2 (`self.EditorPlayerStart`))
  (:`Pressed`
    (`|ExecutionSequence`
      (:`then_0`
        (`|ExecutionSequence`
          (:`then_0`
            ;[1 1 1] Foliage Painting
            (`/Engine/EditorBlueprintResources/StandardMacros.IsValid` (`self.EditorPaintBrush`)
              (:`Is Valid`
                (`/Game/MapEditorExample/Blueprints/Misc/BP_PaintBrush.StartPainting` (`self.EditorPaintBrush`)))))
          (:`then_1`
            (`self.RemoveColorButtons`))))
      (:`then_1`
        (`/Engine/EditorBlueprintResources/StandardMacros.IsValid` _editorpaintbrush
          (:`Is Not Valid`
            (`self.CloseGate`)
            (`|ExecutionSequence`
              (:`then_0`
                (`/Engine/EditorBlueprintResources/StandardMacros.IsValid` _previewbuilding
                  (:`Is Valid`
                    (`self.SpawnBuildingInWorld` (castclass `/Game/MapEditorExample/Blueprints/Buildings/BP_MasterBuilding` (`GameplayStatics.GetObjectClass` _previewbuilding) :!pure true) false (`self.PreviewBuildingLocation`))
                    (`/Game/MapEditorExample/Blueprints/HUD/EditorHUD.SetWidgetEnableState` (`self.EditorHUD`) true))))
              (:`then_1`
                (`/Engine/EditorBlueprintResources/StandardMacros.IsValid` _editorplayerstart
                  (:`Is Valid`
                    (if (not (`/Game/MapEditorExample/Blueprints/Misc/BP_PlayerStart.bCanBeMoved` _editorplayerstart))
                      (`self.K2_SetActorLocation` _editorplayerstart (`self.PreviewBuildingLocation`) false)
                      (`/Game/MapEditorExample/Blueprints/HUD/EditorHUD.SetWidgetEnableState` (`self.EditorHUD`) true)
                      (`/Game/MapEditorExample/Blueprints/HUD/EditorHUD.PlayerStartSet` (`self.EditorHUD`))))))))))))
  (:`Released`
    (`|ExecutionSequence`
      (:`then_0`
        (`/Engine/EditorBlueprintResources/StandardMacros.IsValid` _editorpaintbrush
          (:`Is Valid`
            (`/Game/MapEditorExample/Blueprints/Misc/BP_PaintBrush.StopPainting` _editorpaintbrush))))
      (:`then_1`
        (`/Engine/EditorBlueprintResources/StandardMacros.IsValid` _editorplayerstart_2
          (:`Is Valid`
            (`/Game/MapEditorExample/Blueprints/Misc/BP_PlayerStart.ActivateMovementMode` _editorplayerstart_2)))))))

(event `self.ActivatePlayMode`
  (bind _editorplayerstart (`self.EditorPlayerStart`))
  ;[1 1 1] Interface Event: Start Playing
  (`GameplayStatics.PlaySoundAtLocation` "/Engine/EditorSounds/GamePreview/StartSimulate_Cue.StartSimulate_Cue" (`self.K2_GetActorLocation` (`self.EditorCamera`)))
  (`self.CloseGate`)
  (`|ExecutionSequence`
    (:`then_0`
      (`/Game/MapEditorExample/Blueprints/HUD/EditorHUD.RemoveColorButtons` (`self.EditorHUD`)))
    (:`then_1`
      (set `self.bShowMouseCursor` false))
    (:`then_2`
      (set `self.bIsSpectating` false))
    (:`then_3`
      (`/Game/MapEditorExample/Blueprints/Misc/BP_PlayerStart.ActivatePlayMode` _editorplayerstart true)
      (`/Engine/EditorBlueprintResources/StandardMacros.IsValid` (`self.EditorCharacter`)
        (:`Is Valid`
          (`self.Possess` (`self.EditorCharacter`)))
        (:`Is Not Valid`
          (bind _returnvalue (`|SpawnActorFromClass` "/Game/MapEditorExample/Blueprints/BP_EditorCharacter.BP_EditorCharacter_C" (`SceneComponent.K2_GetComponentToWorld` (`/Game/MapEditorExample/Blueprints/Misc/BP_PlayerStart.PlayerSpawnArrow` _editorplayerstart))))
          (bind _output_get (set `self.EditorCharacter` _returnvalue))
          (`self.Possess` _output_get))))))

(event `InputAxis|MoveForward` :consume false
  (params (AxisValue :type "Float (single-precision)"))
  (set `/Game/MapEditorExample/Blueprints/BP_EditorCamera.ForwardAxis` AxisValue (`self.EditorCamera`)))

(event `InputAction|ExitFoliageBrush`
  ;[1 1 1] Exit Foliage Mode
  (:`Pressed`
    (`self.CloseGate`)
    (`self.K2_DestroyActor` (`self.EditorPaintBrush`))
    (set `self.EditorPaintBrush` null)
    (`/Game/MapEditorExample/Blueprints/HUD/EditorHUD.SetWidgetEnableState` (`self.EditorHUD`) true)))

(event `InputAxis|MoveRight` :consume false
  (params (AxisValue :type "Float (single-precision)"))
  (set `/Game/MapEditorExample/Blueprints/BP_EditorCamera.RightAxis` AxisValue (`self.EditorCamera`)))

(event `self.ActivatePauseMode`
  (bind _editorcamera (`self.EditorCamera`))
  ;[1 1 1] Interface Event: Pause playing (Eject player)
  (set `self.bIsSpectating` true)
  (switch `/Game/MapEditorExample/Blueprints/Enums/ECameraMode` (`/Game/MapEditorExample/Blueprints/BP_EditorCamera.GetCameraMode` (`self.EditorCamera`))
    (:`NewEnumerator0`
      (`self.UnPossess`)
      (`self.Possess` (`self.DefaultPawn`)))
    (:`NewEnumerator1`
      (`self.SetCamera` _editorcamera)))
  (`GameplayStatics.PlaySoundAtLocation` "/Engine/EditorSounds/GamePreview/EjectFromPlayer_Cue.EjectFromPlayer_Cue" (`self.K2_GetActorLocation` _editorcamera))
  (set `self.bShowMouseCursor` true))

(event `self.ReceiveBeginPlay`
  ;[1 1 1] Add HUD
  (bind _returnvalue (`|CreateWidget` "/Game/MapEditorExample/Blueprints/HUD/EditorHUD.EditorHUD_C" self))
  (bind _output_get (set `self.EditorHUD` _returnvalue))
  (`UserWidget.AddToViewport` _output_get))

(event `InputAxis|Turn` :consume false
  (params (AxisValue :type "Float (single-precision)"))
  (bind _editorcamera (`self.EditorCamera`))
  (if (`self.IsInputKeyDown` "RightMouseButton")
    (`self.SetActorRotation` _editorcamera (`KismetMathLibrary.MakeRot` (.pitch (`self.K2_GetActorRotation` _editorcamera)) (+ (.yaw (`self.K2_GetActorRotation` _editorcamera)) (* AxisValue (`/Game/MapEditorExample/Blueprints/BP_EditorCamera.RotationSpeed` _editorcamera))) (.roll (`self.K2_GetActorRotation` _editorcamera))))))

(event `self.ActivateStopMode`
  (bind _editorcamera (`self.EditorCamera`))
  ;[1 1 1] Interface Event: Stop Playing (Unpossess and destroy the character)
  (if (not (`self.bIsSpectating`))
    (switch `/Game/MapEditorExample/Blueprints/Enums/ECameraMode` (`/Game/MapEditorExample/Blueprints/BP_EditorCamera.GetCameraMode` _editorcamera)
      (:`NewEnumerator0`
        (`self.UnPossess`)
        (`self.Possess` (`self.DefaultPawn`)))
      (:`NewEnumerator1`
        (`self.SetCamera` _editorcamera :!pinned true) ; This thing is not working. Any idea why?
      )))
  (`self.K2_DestroyActor` (`self.EditorCharacter`))
  (set `self.EditorCharacter` null)
  (`GameplayStatics.PlaySoundAtLocation` "/Engine/EditorSounds/GamePreview/EndSimulate_Cue.EndSimulate_Cue" (`self.K2_GetActorLocation` (`self.EditorCamera`)))
  (`/Game/MapEditorExample/Blueprints/Misc/BP_PlayerStart.ActivatePlayMode` (`self.EditorPlayerStart`) false)
  (set `self.bShowMouseCursor` true))

(event `self.SetCamera`
  (params (EditorCamera :type "/Game/MapEditorExample/Blueprints/BP_EditorCamera Object Reference"))
  (bind _editorcamera (`self.EditorCamera`))
  ;[1 1 1] Interface Event: Switch camera (RTS mode only)
  (`/Engine/EditorBlueprintResources/StandardMacros.IsValid` _editorcamera
    (:`Is Valid`
      (`self.SetViewTargetWithBlend` _editorcamera 0.0 "VTBlend_Cubic"))
    (:`Is Not Valid`
      (bind _output_get (set `self.EditorCamera` EditorCamera))
      (`self.SetViewTargetWithBlend` _output_get 0.0 "VTBlend_Cubic"))))

(event `self.PossessDefaultPawn`
  (params (Pawn :type "DefaultPawn Object Reference"))
  ;[1 1 1] Interface Event: Possess default pawn (Free cam mode only)
  (`self.Possess` Pawn)
  (bind _output_get (set `self.DefaultPawn` Pawn))
  (`self.SetActorHiddenInGame` _output_get true))

(fn `RemoveColorButtons`
  (if (not (`KismetMathLibrary.ClassIsChildOf` (`GameplayStatics.GetObjectClass` (`.HitActor` (`GameplayStatics.BreakHitResult` (`self.GetHitResultUnderCursorByChannel` "TraceTypeQuery1")))) "/Game/MapEditorExample/Blueprints/Buildings/BP_MasterBuilding.BP_MasterBuilding_C"))
    (`/Game/MapEditorExample/Blueprints/HUD/EditorHUD.RemoveColorButtons` (`self.EditorHUD`)))
  (return))

(fn `SpawnBuildingInWorld`
  (params (BuildingClass :type "/Game/MapEditorExample/Blueprints/Buildings/BP_MasterBuilding Class Reference") (bPreviewMode :type Boolean :default false) (SpawnLocation :type "Object.Vector Structure" :default (0.0 0.0 0.0)))
  (bind _returnvalue (`|SpawnActorFromClass` BuildingClass (`KismetMathLibrary.MakeTransform` SpawnLocation)))
  (`|ExecutionSequence`
    (:`then_0`
      (`/Game/MapEditorExample/Blueprints/Buildings/BP_MasterBuilding.PreviewMode` _returnvalue bPreviewMode))
    (:`then_1`
      (if bPreviewMode
        (set `self.PreviewBuilding` _returnvalue)
        (else
          (`self.K2_DestroyActor` (`self.PreviewBuilding`)))))
    (:`then_2`
      (if bPreviewMode
        (`self.OpenGate`)))))

(fn `UserConstructionScript`)